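; Collectable coin pickup actor that awards points to the player's ThirdPersonCharacter.
; When the player pawn overlaps it, it plays a pickup sound, spawns a particle effect at its sphere, destroys itself, then increases the character's Point value.
; Tick spins the actor around Z and calls Play on the Bob timeline, whose updates apply local offsets for up-and-down movement.
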(event Collision|EventActorBeginOverlap
  (params (OtherActor :type Actor%20Object%20Reference))
  ;[0.08438 0.3916 0.08438] We check there if the Third Person Character enters the Sphere Collision the Actor destroys itself (Before that we check if the Actor who enters the Sphere Collision is our Third Person Character, if yes then actor Destroys itself)
  (if (== OtherActor (Game|Player|GetPlayerPawn 0))
    (Audio|PlaySound2D "/Game/SoundEffects/CoinPickUpSound.CoinPickUpSound" 1.0 1.0 0.0 0 0)
    (Effects|SpawnEmitteratLocation "/Game/Particles/p_collectable.p_collectable" (Transformation|GetWorldLocation (Variables|Default|GetSphere)))
    (Actor|DestroyActor)
    (bind _asthird_person_character (Utilities|Casting|CastToThirdPersonCharacter (Game|Player|GetPlayerPawn 0)))
    (Variables|/Game/ThirdPersonBP/Blueprints/ThirdPersonCharacter.ThirdPersonCharacter_C|SetPoint _asthird_person_character (+ (Variables|/Game/ThirdPersonBP/Blueprints/ThirdPersonCharacter.ThirdPersonCharacter_C|GetPoint _asthird_person_character) 10))))

(event EventTick
  (params (DeltaSeconds :type Float%20%28single-precision%29))
  ;[0.6308 0.2623 0.07619] Allows us to turn the Actor around Z axis
  (Transformation|AddActorLocalRotation "0,3.000000, 0" false false)
  (bind _newtrack_0 (Timeline|Bob Play)
    (:Update
      ;[1 0.3075 0.3872] This allows us to set the object (so it can move up&down)
      (Transformation|AddActorLocalOffset _newtrack_0 false false))))

(fn ConstructionScript)